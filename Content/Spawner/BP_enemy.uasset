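; BP_enemy is an enemy actor that advances in a straight line toward a hard-coded player position and dies after repeated hits.
; BeginPlay caches the spawn location and that fixed target.
; Tick, throttled by a Delay, teleports it by a constant fraction of the initial offset, without sweep or stopping at the target.
; Any Hit event prints Life, then subtracts fixed damage or destroys the actor when Life would run out.
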(event `self.ReceiveBeginPlay`
  (set `self.Life` 20)
  (set `self.PlayerPos` (-104.0 1338.0 912.0))
  (bind _output_get (set `self.InitialEnemyPos` (`self.K2_GetActorLocation`)))
  (set `self.RecentEnemyPos` _output_get))

(event `self.ReceiveHit`
  (params (MyComp :type "PrimitiveComponent Object Reference") (Other :type "Actor Object Reference") (OtherComp :type "PrimitiveComponent Object Reference") (bSelfMoved :type Boolean) (HitLocation :type "Vector Structure") (HitNormal :type "Vector Structure") (NormalImpulse :type "Vector Structure") (Hit :type "HitResult Structure (by ref)"))
  (bind _life (`self.Life`))
  (bind _returnvalue (- _life 10))
  (`KismetSystemLibrary.PrintString` (`KismetStringLibrary.Conv_IntToString` _life))
  (if (> _returnvalue 0)
    (set `self.Life` _returnvalue)
    (else
      (`self.K2_DestroyActor`))))

(event `self.ReceiveTick`
  (params (DeltaSeconds :type "Float (single-precision)"))
  (`KismetSystemLibrary.Delay` 0.2)
  (bind _output_get (set `self.RecentEnemyPos` (+ (`self.RecentEnemyPos`) (* (- (`self.InitialEnemyPos`) (`self.PlayerPos`)) -0.01))))
  (`self.K2_SetActorLocation` _output_get))

(fn `UserConstructionScript`)