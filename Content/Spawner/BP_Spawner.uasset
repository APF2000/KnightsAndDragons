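; BP_Spawner is a spawner actor that keeps a single BP_Enemy in the world, replacing it once it is no longer valid.
; It attempts a spawn on BeginPlay and again roughly every 10 seconds through a Delay on Tick.
; AttemptToSpawn checks the stored Enemy reference, and SpawnEnemy creates a replacement at the spawner's location and rotation, adjusting for collisions but always spawning.
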(event `self.ReceiveBeginPlay`
  (`self.AttemptToSpawn` :!label _label))

(event `self.ReceiveTick`
  (params (DeltaSeconds :type "Float (single-precision)"))
  (`KismetSystemLibrary.Delay` 10.0)
  (goto _label))

(fn `AttemptToSpawn`
  (`/Engine/EditorBlueprintResources/StandardMacros.IsValid` (`self.Enemy`)
    (:`Is Not Valid`
      (`self.SpawnEnemy`))))

(fn `SpawnEnemy`
  (bind _returnvalue (`|SpawnActorFromClass` "/Game/Spawner/BP_enemy.BP_Enemy_C" (`KismetMathLibrary.MakeTransform` (`self.K2_GetActorLocation`) (`self.K2_GetActorRotation`)) "AdjustIfPossibleButAlwaysSpawn" "OverrideRootScale" null null))
  (set `self.Enemy` _returnvalue))

(fn `UserConstructionScript`)